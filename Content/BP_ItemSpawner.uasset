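; BP_ItemSpawner is a box-volume spawner that scatters BP_Item pickups at random points when play begins on a dedicated server.
; After a short delay it caches BP_My_GameState, then spawns a few items of that state's current item type plus several surrogate decoys.
; Surrogates draw a random type from a list with the game state's type removed.
; The construction script sizes the box from an extent variable.
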(event `self.ReceiveBeginPlay`
  ; Server
  (if (`KismetSystemLibrary.IsDedicatedServer`)
    (`KismetSystemLibrary.Delay` 1.0)
    (`self.SpawnItems_Server`)
    (bind _asbp_my_game_state (cast `/Game/BP_My_GameState` (`GameplayStatics.GetGameState`)))
    (set `self.As BP My Game State` _asbp_my_game_state)
    (for _ (range 1 3)
      (`self.SpawnItems_Server`))
    (for _ (range 1 6)
      (`self.SpawnSurrogate_Server`))))

(event `SpawnItems_Server`
  (bind _as_bp_my_game_state (`self.As BP My Game State`))
  ; Not RPC
  (`/Engine/EditorBlueprintResources/StandardMacros.IsValid` _as_bp_my_game_state
    (:`Is Valid`
      (`|SpawnActorFromClass` "/Game/BP_Item.BP_Item_C" (`KismetMathLibrary.MakeTransform` (`KismetMathLibrary.RandomPointInBoundingBox` (`self.K2_GetActorLocation`) (`BoxComponent.GetScaledBoxExtent` (`self.Box`)))) "AlwaysSpawn" "MultiplyWithRoot" null (`/Game/BP_My_GameState.EMyItems` _as_bp_my_game_state) null))))

(event `SpawnSurrogate_Server`
  (bind _as_bp_my_game_state (`self.As BP My Game State`))
  ; Not RPC
  (`/Engine/EditorBlueprintResources/StandardMacros.IsValid` _as_bp_my_game_state
    (:`Is Valid`
      (`KismetArrayLibrary.Array_RemoveItem` (`self.SurogateItemTypes`) (`/Game/BP_My_GameState.EMyItems` _as_bp_my_game_state))
      (`|SpawnActorFromClass` "/Game/BP_Item.BP_Item_C" (`KismetMathLibrary.MakeTransform` (`KismetMathLibrary.RandomPointInBoundingBox` (`self.K2_GetActorLocation`) (`BoxComponent.GetScaledBoxExtent` (`self.Box`)))) "AlwaysSpawn" "MultiplyWithRoot" null (`KismetArrayLibrary.Array_Random` (`self.SurogateItemTypes`)) null))))

(fn `UserConstructionScript`
  (`BoxComponent.SetBoxExtent` (`self.Box`) (`self.In Box Extent`) true))