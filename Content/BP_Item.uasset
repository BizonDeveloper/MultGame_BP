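; Collectible item actor that adds to a count in BP_My_GameState when interacted with, if it is the matching type.
; On BeginPlay, only on a dedicated server, it caches the game state and sets a cube, sphere or cylinder mesh from ItemType.
; Interact compares ItemType to the game state's EMyItems, then calls AddCurrentItemCountServer, noted as not an RPC, and destroys the actor.
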(event `self.ReceiveBeginPlay`
  ; Server
  (if (`KismetSystemLibrary.IsDedicatedServer`)
    (bind _asbp_my_game_state (cast `/Game/BP_My_GameState` (`GameplayStatics.GetGameState`)))
    (set `self.As BP My Game State` _asbp_my_game_state)
    (`StaticMeshComponent.SetStaticMesh` (`self.StaticMesh`) (select `/Game/E_MyItems` (`self.ItemType`) :`NewEnumerator0` "/Game/ThirdPerson/Maps/_GENERATED/user/SM_ItemCube.SM_ItemCube" :`NewEnumerator1` "/Game/ThirdPerson/Maps/_GENERATED/user/SM_SphereItem.SM_SphereItem" :`NewEnumerator2` "/Game/ThirdPerson/Maps/_GENERATED/user/SM_CilinderItem.SM_CilinderItem" :!type "StaticMesh Object Reference"))))

(event `/Game/BPI_InteractInterface.Interact`
  (params (Interactor :type "Actor Object Reference"))
  (if (`|EnumEquality` (`self.ItemType`) (`/Game/BP_My_GameState.EMyItems` (`self.As BP My Game State`)))
    ; Not Rpc
    (`/Game/BP_My_GameState.AddCurrentItemCount_Server` (`self.As BP My Game State`) 1)
    (`self.K2_DestroyActor`)))

(fn `UserConstructionScript`)