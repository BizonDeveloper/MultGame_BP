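; AC_Interact is an actor component that detects what the owning BP_ThirdPersonCharacter is facing, as a basis for interaction.
; On BeginPlay it caches the owner and starts a looping half-second timer instead of using Tick.
; Each pulse sphere-traces a short distance from the Head socket along the follow camera's forward vector, with debug drawing on.
; It stores the blocking hit in HitActor or clears it; no interaction action is implemented here.
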(event `self.ReceiveBeginPlay`
  (bind _asbp_third_person_character (cast `/Game/BP_ThirdPersonCharacter` (`self.GetOwner`)))
  (set `self.As BP Third Person Character` _asbp_third_person_character)
  (`KismetSystemLibrary.K2_SetTimerDelegate` (delegate `InteractTick`) 0.5 true))

(event `InteractTick`
  (bind _as_bp_third_person_character (`self.As BP Third Person Character`))
  (bind _returnvalue (`SceneComponent.GetSocketLocation` (`Character.Mesh` _as_bp_third_person_character) "Head"))
  (bind _outhit (`KismetSystemLibrary.SphereTraceSingle` :`Start` _returnvalue :`End` (+ _returnvalue (* (`SceneComponent.GetForwardVector` (`/Game/BP_ThirdPersonCharacter.FollowCamera` _as_bp_third_person_character)) 200.0)) :`Radius` 30.0 :`TraceChannel` "TraceTypeQuery1" :`DrawDebugType` "ForDuration"))
  (bind (_bblockinghit _binitialoverlap _time _distance _location _impactpoint _normal _impactnormal _physmat _hitactor) (`GameplayStatics.BreakHitResult` _outhit))
  (if _bblockinghit
    (set `self.Hit Actor` _hitactor)
    (else
      (set `self.Hit Actor` null))))