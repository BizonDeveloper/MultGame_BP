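; BP_Door is an interactable door that swings open and closed on successive interactions.
; Interact runs only on a dedicated server, where a FlipFlop alternates between open and close multicast calls.
; The multicast events play or reverse a timeline that lerps the static mesh's relative yaw between closed and a quarter turn open.
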(event `/Game/BPI_InteractInterface.Interact`
  (params (Interactor :type "Actor Object Reference"))
  (if (`KismetSystemLibrary.IsDedicatedServer`)
    (`/Engine/EditorBlueprintResources/StandardMacros.FlipFlop`
      (:`A`
        (`self.OpenDoor_Multicast`))
      (:`B`
        (`self.CloseDoor_Multicast`)))))

(event `OpenDoor_Multicast`
  ; Add Reliable
  (bind (_direction _newtrack_0) (`Timeline|OpendoorTimline` :!label _label)
    (:`Update`
      (`SceneComponent.K2_SetRelativeRotation` (`self.StaticMesh`) (`KismetMathLibrary.MakeRotator` 0.0 0.0 (`KismetMathLibrary.Lerp` 0.0 90.0 _newtrack_0)) false false))))

(event `CloseDoor_Multicast`
  ; Add Reliable
  (goto _label :!via `Reverse`))

(fn `UserConstructionScript`)