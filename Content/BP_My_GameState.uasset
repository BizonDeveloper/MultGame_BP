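; Game state for a multiplayer item-collection round, picking a random item type and target count on begin play.
; A one-second looping timer counts down and ends the round in a win when the count reaches the target, or defeat at zero.
; Multicasts draw the result widget on the local player's character, then a ServerTravel restarts the map.
; RepNotify variables pass time, item type and counts on through update calls.
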(event `self.ReceiveBeginPlay`
  (bind _returnvalue (`KismetSystemLibrary.K2_SetTimerDelegate` (delegate `TickSec`) 1.0 true))
  (set `self.Tickhandle` _returnvalue)
  (`self.Initialize_MyItems_Server`)
  (`self.InitMaxItemCount_Server`))

(event `TickSec`
  (`self.Tick_Server`))

(event `Tick_Server`
  (`/Engine/EditorBlueprintResources/StandardMacros.DecrementInt` (`self.TimeToEnd`)
    (:`  `
      (if (== (`self.CurrentItemCount`) (`self.MaxItemCount`))
        (`self.Win_Multicast`)
        (`KismetSystemLibrary.K2_ClearAndInvalidateTimerHandle` (`self.Tickhandle`))
        (`KismetSystemLibrary.Delay` 2.0)
        (`self.RestartGAme_Server`)
        (elif (== (`self.TimeToEnd`) 0)
          (`KismetSystemLibrary.K2_ClearAndInvalidateTimerHandle` (`self.Tickhandle`))
          (`self.DefeatWidget_Multicast`)
          (`KismetSystemLibrary.Delay` 2.0)
          (`self.RestartGAme_Server`))))))

(event `RestartGame_Server`
  (`KismetSystemLibrary.ExecuteConsoleCommand` "ServerTravel  ThirdPersonMap?listen" null))

(event `Initialize_MyItems_Server`
  (set `self.EMyItems` (`KismetArrayLibrary.Array_Random` (`|MakeArray` "NewEnumerator0" "NewEnumerator1" "NewEnumerator2" :!type "/Game/E_MyItems Enum"))))

(event `DefeatWidget_Multicast`
  (bind _asbp_third_person_character (cast `/Game/BP_ThirdPersonCharacter` (`Controller.K2_GetPawn` (`GameplayStatics.GetPlayerController` 0))))
  (`/Game/BP_ThirdPersonCharacter.DrawDefeatWidget` _asbp_third_person_character))

(event `InitMaxItemCount_Server`
  (set `self.MaxItemCount` (`KismetMathLibrary.RandomIntegerInRange` 3 5)))

(event `Win_Multicast`
  (bind _asbp_third_person_character (cast `/Game/BP_ThirdPersonCharacter` (`Controller.K2_GetPawn` (`GameplayStatics.GetPlayerController` 0))))
  (`/Game/BP_ThirdPersonCharacter.DrawWinWidget` _asbp_third_person_character))

(event `AddCurrentItemCount_Server`
  (params (NewCount :type Integer))
  (set `self.CurrentItemCount` (+ NewCount (`self.CurrentItemCount`))))

(fn `OnRep_CurrentItemCount`
  (`self.UpdateCurrentCountItem` (`self.CurrentItemCount`))
  (return))

(fn `OnRep_EMyItems`
  (`self.UpdateItemTipe` (`self.EMyItems`))
  (return))

(fn `OnRep_MaxItemCount`
  (`self.UpdateMaxCountItem` (`self.MaxItemCount`))
  (return))

(fn `OnRep_TimeToEnd`
  (`self.SecChanged` (`self.TimeToEnd`))
  (return))

(fn `UserConstructionScript`)